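; Game instance for God of Weapon that holds player stats, customization data, coins and run totals.
; LevelUpPlayer scales combat, movement and recovery stats by the current stage's DT_PlayerLevel multiplier, refills HP to the new maximum and randomly grows inventory columns or rows.
; UpdateStageClear saves the player's stats and coins, then accumulates earned coins, damage and monsters defeated.
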(fn `LevelUpPlayer`
  (bind (_playerstat_currenthp _playerstat_maxhp _playerstat_shortrangeattackforce _playerstat_longrangeattackforce _playerstat_attackspeedmultifier _playerstat_movespeedmultifier _playerstat_attackrangemultifier _playerstat_recovery) (break `PlayerStatStructure` (`self.PlayerStat`)))
  (bind _returnvalue (`|GetDataTableRow` "/Game/Blueprints/Data/DataTable/DT_PlayerLevel.DT_PlayerLevel" (`KismetStringLibrary.Conv_StringToName` (`KismetStringLibrary.Conv_IntToString` (`self.CurrentStage`))))
    (:`then`
      (bind _returnvalue_2 (`KismetMathLibrary.FTrunc` (* _playerstat_maxhp (break `/Game/Blueprints/Data/Structure/S_PlayerLevel` _returnvalue))))
      (set `self.PlayerStat` (make `PlayerStatStructure` _returnvalue_2 _returnvalue_2 (`KismetMathLibrary.FTrunc` (* (break `/Game/Blueprints/Data/Structure/S_PlayerLevel` _returnvalue) _playerstat_shortrangeattackforce)) (`KismetMathLibrary.FTrunc` (* (break `/Game/Blueprints/Data/Structure/S_PlayerLevel` _returnvalue) _playerstat_longrangeattackforce)) (* (break `/Game/Blueprints/Data/Structure/S_PlayerLevel` _returnvalue) _playerstat_attackspeedmultifier) (* (break `/Game/Blueprints/Data/Structure/S_PlayerLevel` _returnvalue) _playerstat_movespeedmultifier) (* (break `/Game/Blueprints/Data/Structure/S_PlayerLevel` _returnvalue) _playerstat_attackrangemultifier) (`KismetMathLibrary.FTrunc` (* (break `/Game/Blueprints/Data/Structure/S_PlayerLevel` _returnvalue) _playerstat_recovery))))
      (`/Engine/EditorBlueprintResources/StandardMacros.IncrementInt` (select `bool` (`KismetMathLibrary.RandomBool`) :`false` (`self.InventoryRows`) :`true` (`self.InventoryColumes`))))))

(fn `UpdatePlayerCustomData`
  (params (InPlayerCustomData :type "/Game/Blueprints/Data/Structure/S_CustomizeData Structure"))
  (set `self.PlayerCustomData` InPlayerCustomData))

(fn `UpdateStageClear`
  (params (InPlayerStat :type "PlayerStatStructure Structure") (InPlayerCoin :type Integer) (InPlayerEarnedCoin :type Integer) (InTotalDamage :type Integer) (InTotalMonsterDefeated :type Integer))
  (`|ExecutionSequence`
    (:`then_0`
      (set `self.PlayerStat` InPlayerStat))
    (:`then_1`
      (set `self.PlayerCoin` InPlayerCoin))
    (:`then_2`
      (set `self.PlayerEarnedCoin` (+ (`self.PlayerEarnedCoin`) InPlayerEarnedCoin)))
    (:`then_3`
      (set `self.TotalDamage` (+ (`self.TotalDamage`) InTotalDamage)))
    (:`then_4`
      (set `self.TotalMonsterDefeated` (+ (`self.TotalMonsterDefeated`) InTotalMonsterDefeated)))))