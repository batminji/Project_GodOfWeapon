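; BP_Player is the player Blueprint, handling monster damage and death, modular appearance, and equipped items.
; Only hits from MonsterAttack-tagged causers lower HP; reaching zero sets IsDead and calls OnPlayerDie.
; Customization swaps five body-part skeletal meshes from DataTables using blocking loads.
; Each non-consumable inventory item is loaded from DT_ItemData, then spawned as a child actor on its own lagging, randomly yawed spring arm and initialized as a BaseItemActor.
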(event `self.ReceiveAnyDamage`
  (params (Damage :type "Float (single-precision)") (DamageType :type "DamageType Object Reference") (InstigatedBy :type "Controller Object Reference") (DamageCauser :type "Actor Object Reference"))
  (bind _returnvalue_currenthp (break `PlayerStatStructure` (`self.GetCurrentPlayerStat`)))
  (bind (_returnvalue_currenthp_2 _returnvalue_maxhp _returnvalue_shortrangeattackforce _returnvalue_longrangeattackforce _returnvalue_attackspeedmultifier _returnvalue_movespeedmultifier _returnvalue_attackrangemultifier _returnvalue_recovery) (break `PlayerStatStructure` (`self.GetCurrentPlayerStat`)))
  (if (`self.bIsDead`)
    _
    (elif (`self.ActorHasTag` DamageCauser "MonsterAttack")
      (`self.SetCurrentPlayerStat` (make `PlayerStatStructure` (- _returnvalue_currenthp_2 Damage) _returnvalue_maxhp _returnvalue_shortrangeattackforce _returnvalue_longrangeattackforce _returnvalue_attackspeedmultifier _returnvalue_movespeedmultifier _returnvalue_attackrangemultifier _returnvalue_recovery))
      (if (<= _returnvalue_currenthp 0)
        (set `self.bIsDead` true)
        (`self.SetCurrentPlayerStat` (make `PlayerStatStructure` 0))
        (`self.OnPlayerDie`)))))

(event `self.UpdatePlayerCustom`
  (params (InCustomData :type "CustomData Structure (by ref)"))
  (`|ExecutionSequence`
    (:`then_0`
      (bind _returnvalue (`|GetDataTableRow` "/Game/Blueprints/Data/DataTable/Customize/DT_CustomHead.DT_CustomHead" (`KismetStringLibrary.Conv_StringToName` (`KismetStringLibrary.Conv_IntToString` InCustomData_HeadNumber)))
        (:`then`
          (`KismetSystemLibrary.LoadAsset_Blocking` (`.SkeletalMesh_18_3184F0D441A03C2D2BFF438050DA58D0` (break `/Game/Blueprints/Data/Structure/S_CustomizeMesh` _returnvalue)))
          (`SkeletalMeshComponent.SetSkeletalMeshAsset` (`self.Head`) (`|ConvertAsset` (`.SkeletalMesh_18_3184F0D441A03C2D2BFF438050DA58D0` (break `/Game/Blueprints/Data/Structure/S_CustomizeMesh` _returnvalue)))))))
    (:`then_1`
      (bind _returnvalue_2 (`|GetDataTableRow` "/Game/Blueprints/Data/DataTable/Customize/DT_CustomChest.DT_CustomChest" (`KismetStringLibrary.Conv_StringToName` (`KismetStringLibrary.Conv_IntToString` InCustomData_ChestNumber)))
        (:`then`
          (`KismetSystemLibrary.LoadAsset_Blocking` (`.SkeletalMesh_18_3184F0D441A03C2D2BFF438050DA58D0` (break `/Game/Blueprints/Data/Structure/S_CustomizeMesh` _returnvalue_2)))
          (`SkeletalMeshComponent.SetSkeletalMeshAsset` (`self.Chest`) (`|ConvertAsset` (`.SkeletalMesh_18_3184F0D441A03C2D2BFF438050DA58D0` (break `/Game/Blueprints/Data/Structure/S_CustomizeMesh` _returnvalue_2)))))))
    (:`then_2`
      (bind _returnvalue_3 (`|GetDataTableRow` "/Game/Blueprints/Data/DataTable/Customize/DT_CustomHands.DT_CustomHands" (`KismetStringLibrary.Conv_StringToName` (`KismetStringLibrary.Conv_IntToString` InCustomData_HandsNumber)))
        (:`then`
          (`KismetSystemLibrary.LoadAsset_Blocking` (`.SkeletalMesh_18_3184F0D441A03C2D2BFF438050DA58D0` (break `/Game/Blueprints/Data/Structure/S_CustomizeMesh` _returnvalue_3)))
          (`SkeletalMeshComponent.SetSkeletalMeshAsset` (`self.Hands`) (`|ConvertAsset` (`.SkeletalMesh_18_3184F0D441A03C2D2BFF438050DA58D0` (break `/Game/Blueprints/Data/Structure/S_CustomizeMesh` _returnvalue_3)))))))
    (:`then_3`
      (bind _returnvalue_4 (`|GetDataTableRow` "/Game/Blueprints/Data/DataTable/Customize/DT_CustomLegs.DT_CustomLegs" (`KismetStringLibrary.Conv_StringToName` (`KismetStringLibrary.Conv_IntToString` InCustomData_LegsNumber)))
        (:`then`
          (`KismetSystemLibrary.LoadAsset_Blocking` (`.SkeletalMesh_18_3184F0D441A03C2D2BFF438050DA58D0` (break `/Game/Blueprints/Data/Structure/S_CustomizeMesh` _returnvalue_4)))
          (`SkeletalMeshComponent.SetSkeletalMeshAsset` (`self.Legs`) (`|ConvertAsset` (`.SkeletalMesh_18_3184F0D441A03C2D2BFF438050DA58D0` (break `/Game/Blueprints/Data/Structure/S_CustomizeMesh` _returnvalue_4)))))))
    (:`then_4`
      (bind _returnvalue_5 (`|GetDataTableRow` "/Game/Blueprints/Data/DataTable/Customize/DT_CustomFoot.DT_CustomFoot" (`KismetStringLibrary.Conv_StringToName` (`KismetStringLibrary.Conv_IntToString` InCustomData_FootNumber)))
        (:`then`
          (`KismetSystemLibrary.LoadAsset_Blocking` (`.SkeletalMesh_18_3184F0D441A03C2D2BFF438050DA58D0` (break `/Game/Blueprints/Data/Structure/S_CustomizeMesh` _returnvalue_5)))
          (`SkeletalMeshComponent.SetSkeletalMeshAsset` (`self.Foot`) (`|ConvertAsset` (`.SkeletalMesh_18_3184F0D441A03C2D2BFF438050DA58D0` (break `/Game/Blueprints/Data/Structure/S_CustomizeMesh` _returnvalue_5)))))))))

(event `self.ApplyInventoryItems`
  (params (InItems :type "Array of SavedItemData Structure (by ref)"))
  (for _array_element InItems
    (bind _returnvalue (`|GetDataTableRow` "/Game/Blueprints/Data/DataTable/DT_ItemData.DT_ItemData" (`.ItemRowName` (break `SavedItemData` _array_element)))
      (:`then`
        (if (`|EnumInequality` (`.Type` (break `ItemData` _returnvalue)) "Consume")
          (`KismetSystemLibrary.LoadClassAsset_Blocking` (`.ItemActorClass` (break `ItemData` _returnvalue)))
          (`KismetSystemLibrary.LoadAsset_Blocking` (`.ItemMesh` (break `ItemData` _returnvalue)))
          (`KismetSystemLibrary.LoadAsset_Blocking` (`.ItemNiagara` (break `ItemData` _returnvalue)))
          (`KismetSystemLibrary.LoadAsset_Blocking` (`.ArrowMesh` (break `ItemData` _returnvalue)))
          (`KismetSystemLibrary.LoadAsset_Blocking` (`.ArrowNiagara` (break `ItemData` _returnvalue)))
          ; 플레이어 Attach를 호출
          (`self.AttachItemToPlayer` (`|ConvertAsset` (`.ItemActorClass` (break `ItemData` _returnvalue))) (`.Type` (break `ItemData` _returnvalue)) (`.Stat` (break `ItemData` _returnvalue)) (`|ConvertAsset` (`.ItemMesh` (break `ItemData` _returnvalue))) (`|ConvertAsset` (`.ItemNiagara` (break `ItemData` _returnvalue))) (`|ConvertAsset` (`.ArrowMesh` (break `ItemData` _returnvalue))) (`|ConvertAsset` (`.ArrowNiagara` (break `ItemData` _returnvalue)))))))))

(event `SettingSpringArmComponent`
  (params (InSpringArmRef :type "SpringArmComponent Object Reference"))
  (`|ExecutionSequence`
    (:`then_0`
      (set `SpringArmComponent.TargetArmLength` 120.0 InSpringArmRef))
    (:`then_1`
      (set `SpringArmComponent.CameraLagSpeed` 5.0 InSpringArmRef)
      (set `SpringArmComponent.bEnableCameraLag` true InSpringArmRef)
      (set `SpringArmComponent.bEnableCameraRotationLag` true InSpringArmRef))
    (:`then_2`
      (set `SpringArmComponent.bDoCollisionTest` false InSpringArmRef))))

(fn `AttachItemToPlayer`
  (params (InItemBaseActorClass :type "Actor Class Reference") (InItemType :type "EItemType Enum" :default "Sword") (InItemStat :type "ItemStat Structure") (InItemMesh :type "StaticMesh Object Reference") (InItemNiagara :type "NiagaraSystem Object Reference") (InArrowMesh :type "StaticMesh Object Reference") (InArrowNiagara :type "NiagaraSystem Object Reference"))
  (returns (ReturnValue :type Boolean))
  (locals (SpringArmComponentRef :type "SpringArmComponent Object Reference") (ChidActorComponentRef :type "ChildActorComponent Object Reference"))
  (`|ExecutionSequence`
    (:`then_0`
      ; Spring Arm Attach
      (bind _returnvalue (`AddComponent|NODE_AddSpringArmComponent-1` :`RelativeTransform` (`KismetMathLibrary.MakeTransform` (0.0 0.0 0.0) (`KismetMathLibrary.MakeRotator` 0.0 0.0 (`KismetMathLibrary.RandomFloatInRange` -90.0 90.0)))))
      (bind _output_get (set `local.SpringArmComponentRef` _returnvalue))
      (`self.SettingSpringArmComponent` _output_get)
      (`SceneComponent.K2_AttachToComponent` (`local.SpringArmComponentRef`) (`self.CapsuleComponent`) "None" "SnapToTarget" "SnapToTarget" "SnapToTarget" true))
    (:`then_1`
      ; Child Actor Attach
      (bind _returnvalue_2 (`AddComponent|NODE_AddChildActorComponent-1`))
      (set `local.ChidActorComponentRef` _returnvalue_2)
      (`SceneComponent.K2_AttachToComponent` (`local.ChidActorComponentRef`) (`local.SpringArmComponentRef`) "None" "SnapToTarget" "SnapToTarget" "SnapToTarget" true)
      (`ChildActorComponent.SetChildActorClass` (`local.ChidActorComponentRef`) (`local.InItemBaseActorClass`)))
    (:`then_2`
      ; Attack Item Init
      (bind _asbase_item_actor (cast `BaseItemActor` (`ChildActorComponent.ChildActor` (`local.ChidActorComponentRef`))))
      (`/Engine/EditorBlueprintResources/StandardMacros.IsValid` _asbase_item_actor
        (:`Is Valid`
          (`BaseItemActor.SetPlayer` _asbase_item_actor)
          (`BaseItemActor.InitItem` _asbase_item_actor (`local.InItemType`) (`local.InItemStat`) (`local.SpringArmComponentRef`) (`local.ChidActorComponentRef`) (`local.InItemMesh`) (`local.InItemNiagara`) (`local.InArrowMesh`) (`local.InArrowNiagara`)))))
    (:`then_3`
      (return true))))

(fn `UserConstructionScript`)