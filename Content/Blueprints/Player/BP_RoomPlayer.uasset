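; BP_RoomPlayer is a player character display that applies modular customization to separate head, chest, hands, legs and foot skeletal meshes.
; UpdatePlayerCustom takes a custom data struct and turns each part's number into a row name for that part's DataTable.
; Found rows have their mesh loaded synchronously with LoadAssetBlocking and set on the matching component; missing rows leave that part unchanged.
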(event `self.UpdatePlayerCustom`
  (params (InCustomData :type "CustomData Structure (by ref)"))
  (`|ExecutionSequence`
    (:`then_0`
      (bind _returnvalue (`|GetDataTableRow` "/Game/Blueprints/Data/DataTable/Customize/DT_CustomHead.DT_CustomHead" (`KismetStringLibrary.Conv_StringToName` (`KismetStringLibrary.Conv_IntToString` InCustomData_HeadNumber)))
        (:`then`
          (`KismetSystemLibrary.LoadAsset_Blocking` (`.SkeletalMesh_18_3184F0D441A03C2D2BFF438050DA58D0` (break `/Game/Blueprints/Data/Structure/S_CustomizeMesh` _returnvalue)))
          (`SkeletalMeshComponent.SetSkeletalMeshAsset` (`self.Head`) (`|ConvertAsset` (`.SkeletalMesh_18_3184F0D441A03C2D2BFF438050DA58D0` (break `/Game/Blueprints/Data/Structure/S_CustomizeMesh` _returnvalue)))))))
    (:`then_1`
      (bind _returnvalue_2 (`|GetDataTableRow` "/Game/Blueprints/Data/DataTable/Customize/DT_CustomChest.DT_CustomChest" (`KismetStringLibrary.Conv_StringToName` (`KismetStringLibrary.Conv_IntToString` InCustomData_ChestNumber)))
        (:`then`
          (`KismetSystemLibrary.LoadAsset_Blocking` (`.SkeletalMesh_18_3184F0D441A03C2D2BFF438050DA58D0` (break `/Game/Blueprints/Data/Structure/S_CustomizeMesh` _returnvalue_2)))
          (`SkeletalMeshComponent.SetSkeletalMeshAsset` (`self.Chest`) (`|ConvertAsset` (`.SkeletalMesh_18_3184F0D441A03C2D2BFF438050DA58D0` (break `/Game/Blueprints/Data/Structure/S_CustomizeMesh` _returnvalue_2)))))))
    (:`then_2`
      (bind _returnvalue_3 (`|GetDataTableRow` "/Game/Blueprints/Data/DataTable/Customize/DT_CustomHands.DT_CustomHands" (`KismetStringLibrary.Conv_StringToName` (`KismetStringLibrary.Conv_IntToString` InCustomData_HandsNumber)))
        (:`then`
          (`KismetSystemLibrary.LoadAsset_Blocking` (`.SkeletalMesh_18_3184F0D441A03C2D2BFF438050DA58D0` (break `/Game/Blueprints/Data/Structure/S_CustomizeMesh` _returnvalue_3)))
          (`SkeletalMeshComponent.SetSkeletalMeshAsset` (`self.Hands`) (`|ConvertAsset` (`.SkeletalMesh_18_3184F0D441A03C2D2BFF438050DA58D0` (break `/Game/Blueprints/Data/Structure/S_CustomizeMesh` _returnvalue_3)))))))
    (:`then_3`
      (bind _returnvalue_4 (`|GetDataTableRow` "/Game/Blueprints/Data/DataTable/Customize/DT_CustomLegs.DT_CustomLegs" (`KismetStringLibrary.Conv_StringToName` (`KismetStringLibrary.Conv_IntToString` InCustomData_LegsNumber)))
        (:`then`
          (`KismetSystemLibrary.LoadAsset_Blocking` (`.SkeletalMesh_18_3184F0D441A03C2D2BFF438050DA58D0` (break `/Game/Blueprints/Data/Structure/S_CustomizeMesh` _returnvalue_4)))
          (`SkeletalMeshComponent.SetSkeletalMeshAsset` (`self.Legs`) (`|ConvertAsset` (`.SkeletalMesh_18_3184F0D441A03C2D2BFF438050DA58D0` (break `/Game/Blueprints/Data/Structure/S_CustomizeMesh` _returnvalue_4)))))))
    (:`then_4`
      (bind _returnvalue_5 (`|GetDataTableRow` "/Game/Blueprints/Data/DataTable/Customize/DT_CustomFoot.DT_CustomFoot" (`KismetStringLibrary.Conv_StringToName` (`KismetStringLibrary.Conv_IntToString` InCustomData_FootNumber)))
        (:`then`
          (`KismetSystemLibrary.LoadAsset_Blocking` (`.SkeletalMesh_18_3184F0D441A03C2D2BFF438050DA58D0` (break `/Game/Blueprints/Data/Structure/S_CustomizeMesh` _returnvalue_5)))
          (`SkeletalMeshComponent.SetSkeletalMeshAsset` (`self.Foot`) (`|ConvertAsset` (`.SkeletalMesh_18_3184F0D441A03C2D2BFF438050DA58D0` (break `/Game/Blueprints/Data/Structure/S_CustomizeMesh` _returnvalue_5)))))))))

(fn `UserConstructionScript`)