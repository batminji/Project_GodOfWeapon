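; C_Title is a player controller for the title screen, though its BeginPlay and MoveCamera events are empty.
; Its unconnected graph logic would set the view to the CineCameraActor tagged TitleCamera, with UI-only input and a visible cursor.
; A second unconnected chain would blend to the CustomCamera-tagged camera with easing, wait out the blend, then call OnMoveCameraEnded.
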(event `self.ReceiveBeginPlay`)

(event `MoveCamera`)

(fn `UserConstructionScript`)