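; GM_Inventory is a game mode Blueprint for inventory, with an unfinished item-loading pass.
; Init casts the game instance to BP_GodOfWeaponGameInstance and caches it; BeginPlay is disabled, and nothing here calls Init.
; SetItems loops over the cached instance's InventoryData and looks up each ItemRowName in DT_Items, but does nothing with the rows yet.
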(fn `Init`
  (bind _asbp_god_of_weapon_game_instance (cast `/Game/Blueprints/BP_GodOfWeaponGameInstance` (`GameplayStatics.GetGameInstance`)))
  (`/Engine/EditorBlueprintResources/StandardMacros.IsValid` _asbp_god_of_weapon_game_instance
    (:`Is Valid`
      (set `self.GameInstance` _asbp_god_of_weapon_game_instance))))

(fn `SetItems`
  (for _array_element (`GodOfWeaponGameInstance.InventoryData` (`self.GameInstance`))
    (bind _returnvalue (`|GetDataTableRow` "/Game/Blueprints/Data/DataTable/DT_Items.DT_Items" (`.ItemRowName` (break `SavedItemData` _array_element))))))

(fn `UserConstructionScript`)