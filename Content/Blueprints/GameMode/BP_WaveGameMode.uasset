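; Game mode that sets up the player from saved game instance data when play begins.
; It pushes stored stats and coins to BP_Player, then looks up each inventory item in a data table and blocking-loads every non-consumable's actor class.
; Each item spawns as a child actor on its own lagged, collision-free spring arm attached to the player's capsule, then receives its type and stats.
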(event `self.ReceiveBeginPlay`
  (`self.Init`)
  (`self.UpdatePlayerStat`)
  (`self.SpawnItems`))

(fn `AttachItemToPlayer`
  (params (InItemBaseActorClass :type "BaseItemActor Class Reference") (InItemType :type "EItemType Enum" :default "Sword") (InItemStat :type "ItemStatStructure Structure"))
  (locals (SpringArmComponentRef :type "SpringArmComponent Object Reference") (ChidActorComponentRef :type "ChildActorComponent Object Reference"))
  (`|ExecutionSequence`
    (:`then_0`
      ; Spring Arm Attach
      (bind _returnvalue (`AddComponent|NODE_AddSpringArmComponent-0` :`self` (`self.BP_Player`) :`RelativeTransform` (`KismetMathLibrary.MakeTransform` (0.0 0.0 0.0) (`KismetMathLibrary.MakeRotator` 0.0 0.0 (`KismetMathLibrary.RandomFloatInRange` -90.0 90.0)))))
      (bind _output_get (set `local.SpringArmComponentRef` _returnvalue))
      (`self.SettingSpringArmComponent` _output_get)
      (`SceneComponent.K2_AttachToComponent` (`local.SpringArmComponentRef`) (`Character.CapsuleComponent` (`self.BP_Player`)) "None" "SnapToTarget" "SnapToTarget" "SnapToTarget" true))
    (:`then_1`
      ; Child Actor Attach
      (bind _returnvalue_2 (`AddComponent|NODE_AddChildActorComponent-1` :`self` (`self.BP_Player`)))
      (set `local.ChidActorComponentRef` _returnvalue_2)
      (`SceneComponent.K2_AttachToComponent` (`local.ChidActorComponentRef`) (`local.SpringArmComponentRef`) "None" "SnapToTarget" "SnapToTarget" "SnapToTarget" true)
      (`ChildActorComponent.SetChildActorClass` (`local.ChidActorComponentRef`) (`local.InItemBaseActorClass`)))
    (:`then_2`
      ; Item Init
      (bind _asbp_base_item_actor (cast `/Game/Blueprints/Items/BP_BaseItemActor` (`ChildActorComponent.ChildActor` (`local.ChidActorComponentRef`))))
      (`/Engine/EditorBlueprintResources/StandardMacros.IsValid` _asbp_base_item_actor
        (:`Is Valid`
          (`/Game/Blueprints/Items/BP_BaseItemActor.Init` _asbp_base_item_actor (`local.InItemType`) (`local.InItemStat`)))))))

(fn `Init`
  (bind _asbp_god_of_weapon_game_instance (cast `/Game/Blueprints/BP_GodOfWeaponGameInstance` (`GameplayStatics.GetGameInstance`)))
  (`/Engine/EditorBlueprintResources/StandardMacros.IsValid` _asbp_god_of_weapon_game_instance
    (:`Is Valid`
      (set `self.GameInstance` _asbp_god_of_weapon_game_instance)
      (bind _asbp_player (cast `/Game/Blueprints/Player/BP_Player` (`GameplayStatics.GetPlayerPawn` 0)))
      (`/Engine/EditorBlueprintResources/StandardMacros.IsValid` _asbp_player
        (:`Is Valid`
          (set `self.BP_Player` _asbp_player))))))

(fn `SettingSpringArmComponent`
  (params (InSpringArmRef :type "SpringArmComponent Object Reference"))
  (`|ExecutionSequence`
    (:`then_0`
      (set `SpringArmComponent.TargetArmLength` 120.0 InSpringArmRef))
    (:`then_1`
      (set `SpringArmComponent.CameraLagSpeed` 5.0 InSpringArmRef)
      (set `SpringArmComponent.bEnableCameraLag` true InSpringArmRef)
      (set `SpringArmComponent.bEnableCameraRotationLag` true InSpringArmRef))
    (:`then_2`
      (set `SpringArmComponent.bDoCollisionTest` false InSpringArmRef))))

(fn `SpawnItems`
  (for _array_element (`GodOfWeaponGameInstance.InventoryData` (`self.GameInstance`))
    (bind _returnvalue (`|GetDataTableRow` (`self.DT_Items`) (`.ItemRowName` (break `SavedItemData` _array_element)))
      (:`then`
        (bind (_itemid _type _name _desc _price _itemactorclass _icon _rotateicon _dimension _stat) (break `ItemStructure` _returnvalue))
        (if (`|EnumInequality` _type "Consume")
          (`KismetSystemLibrary.LoadClassAsset_Blocking` _itemactorclass)
          (`self.AttachItemToPlayer` (`|ConvertAsset` _itemactorclass) _type _stat))))))

(fn `UpdatePlayerStat`
  (bind _gameinstance (`self.GameInstance`))
  (bind _bp_player (`self.BP_Player`))
  (`/Engine/EditorBlueprintResources/StandardMacros.IsValid` _bp_player
    (:`Is Valid`
      (`/Game/Blueprints/Player/BP_Player.UpdatePlayerStat` _bp_player (`GodOfWeaponGameInstance.PlayerStat` _gameinstance) (`GodOfWeaponGameInstance.PlayerCoin` _gameinstance)))))

(fn `UserConstructionScript`)