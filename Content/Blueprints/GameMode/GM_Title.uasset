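; Title-screen game mode that runs the pre-game menu flow of title, character customization and level selection, then opens the in-game map.
; Delegates from the C_Title controller and each widget drive the steps, including a camera move after the title widget is removed.
; Customization choices, the starting item, difficulty and its DT_Level multiplier are written to BP_GodOfWeaponGameInstance to carry into gameplay.
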(event `self.ReceiveBeginPlay`
  (bind _asc_title (cast `/Game/Blueprints/Controller/C_Title` (`GameplayStatics.GetPlayerController` 0)))
  (`/Engine/EditorBlueprintResources/StandardMacros.IsValid` _asc_title
    (:`Is Valid`
      (set `self.ControllerRef` _asc_title)
      (add `/Game/Blueprints/Controller/C_Title.OnMoveCameraEnded` _asc_title (`|CreateDelegate` :!event `CreateCustomWidget`))
      (bind _returnvalue (`|CreateWidget` "/Game/UI/Title/WBP_Title.WBP_Title_C"))
      (`UserWidget.AddToViewport` _returnvalue 0)
      (set `self.WBP_Title` _returnvalue)
      (add `/Game/UI/Title/WBP_Title.OnGameStart` _returnvalue (`|CreateDelegate` :!event `MoveCamera`)))))

(event `MoveCamera`
  (bind _wbp_title (`self.WBP_Title`))
  (bind _controllerref (`self.ControllerRef`))
  (`/Engine/EditorBlueprintResources/StandardMacros.IsValid` _wbp_title
    (:`Is Valid`
      (`Widget.RemoveFromParent` _wbp_title)
      (`/Engine/EditorBlueprintResources/StandardMacros.IsValid` _controllerref
        (:`Is Valid`
          (`/Game/Blueprints/Controller/C_Title.MoveCamera` _controllerref))))))

(event `CreateCustomWidget`
  (bind _returnvalue (`|CreateWidget` "/Game/UI/Customize/WBP_Customize.WBP_Customize_C"))
  (`UserWidget.AddToViewport` _returnvalue 0)
  (set `self.WBP_Customize` _returnvalue)
  (add `/Game/UI/Customize/WBP_Customize.OnConfirmCustomize` _returnvalue (`|CreateDelegate` :!event `OnConfirmCustomize`))
  (add `/Game/UI/Customize/WBP_Customize.OnCustomFinishEvent` _returnvalue (`|CreateDelegate` :!event `CreateLevelWidget`)))

(event `OnConfirmCustomize`
  (params (InHeadNumber :type Integer) (InChestNumber :type Integer) (InHandsNumber :type Integer) (InLegsNumber :type Integer) (InFootNumber :type Integer))
  (bind _asbp_god_of_weapon_game_instance (cast `/Game/Blueprints/BP_GodOfWeaponGameInstance` (`GameplayStatics.GetGameInstance`)))
  (`/Game/Blueprints/BP_GodOfWeaponGameInstance.UpdatePlayerCustomData` _asbp_god_of_weapon_game_instance (make `/Game/Blueprints/Data/Structure/S_CustomizeData` InHeadNumber InChestNumber InHandsNumber InLegsNumber InFootNumber)))

(event `CreateLevelWidget`
  (bind _returnvalue (`|CreateWidget` "/Game/UI/Level/WBP_ChooseLevel.WBP_ChooseLevel_C"))
  (`UserWidget.AddToViewport` _returnvalue 0)
  (set `self.WBP_ChooseLevel` _returnvalue)
  (add `/Game/UI/Level/WBP_ChooseLevel.OnStartButtonClicked` _returnvalue (`|CreateDelegate` :!event `StartGame`)))

(event `StartGame`
  (params (InStartItemData :type "SavedItemData Structure") (InLevel :type "EDifficulty Enum" :default "Easy"))
  (`self.UpdateItemAndLevel` InStartItemData InLevel)
  (`GameplayStatics.OpenLevelBySoftObjectPtr` "/Game/Maps/InGameMap.InGameMap"))

(fn `UpdateItemAndLevel`
  (params (NewItem :type "SavedItemData Structure (by ref)") (InputPin :type "EDifficulty Enum" :default "Easy"))
  (bind _asbp_god_of_weapon_game_instance (cast `/Game/Blueprints/BP_GodOfWeaponGameInstance` (`GameplayStatics.GetGameInstance`)))
  (`KismetArrayLibrary.Array_Add` (`GodOfWeaponGameInstance.InventoryData` _asbp_god_of_weapon_game_instance) NewItem)
  (set `GodOfWeaponGameInstance.Difficulty` InputPin _asbp_god_of_weapon_game_instance)
  (bind _returnvalue (`|GetDataTableRow` "/Game/Blueprints/Data/DataTable/DT_Level.DT_Level" (`KismetStringLibrary.Conv_StringToName` (`|GetEnumeratorNameAsString` InputPin)))
    (:`then`
      (set `GodOfWeaponGameInstance.LevelMultiplier` (`.LevelMutiplier_5_5CAF2C334E3EBE9C71126A900491D120` (break `/Game/Blueprints/Data/Structure/S_Level` _returnvalue)) _asbp_god_of_weapon_game_instance))))

(fn `UserConstructionScript`)