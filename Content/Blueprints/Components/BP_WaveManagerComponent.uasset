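; Wave manager component, built on C++ hooks, that runs one timed monster wave and reports stage clear or failure.
; StartGame sets timers for looping spawns, wave end and a player HP recovery, while Tick passes remaining time to the game mode.
; Spawns pull random pooled monsters to reachable points around the player with stat multipliers, capped by alive count.
; Wave end or player death stops spawn and wave timers and returns visible monsters to the pool.
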(event `self.ReceiveBeginPlay`
  (`parent.ReceiveBeginPlay`))

(event `self.SetPlayer`
  ; Set Player CPP
  (bind _asbp_player (cast `/Game/Blueprints/Player/BP_Player` (`GameplayStatics.GetPlayerPawn` 0)))
  (`/Engine/EditorBlueprintResources/StandardMacros.IsValid` _asbp_player
    (:`Is Valid`
      (set `self.InGamePlayer` _asbp_player)
      (add `/Game/Blueprints/Player/BP_Player.OnPlayerDie` _asbp_player (`|CreateDelegate` :!event `OnPlayerDie`)))))

(event `self.ReceiveTick`
  (params (DeltaSeconds :type "Float (single-precision)"))
  (bind _ingamemode (`self.InGameMode`))
  ; Timer Game Mode에 저장
  (`/Engine/EditorBlueprintResources/StandardMacros.IsValid` _ingamemode
    (:`Is Valid`
      (`InGameMode.SetLeftTime` _ingamemode (`KismetSystemLibrary.K2_GetTimerRemainingTimeHandle` (`self.EndWaveTimeHandler`))))))

(event `self.StartGame`
  ; StartGame - CPP
  (bind _returnvalue (`KismetSystemLibrary.K2_SetTimerDelegate` (`|CreateDelegate` :!event `SpawnMonster`) (`self.SpawnInterval`) true))
  (set `self.SpawnMonsterTimeHandler` _returnvalue)
  (bind _returnvalue_2 (`KismetSystemLibrary.K2_SetTimerDelegate` (`|CreateDelegate` :!event `EndWave`) (`self.WaveTimer`)))
  (set `self.EndWaveTimeHandler` _returnvalue_2)
  (bind _returnvalue_3 (`KismetSystemLibrary.K2_SetTimerDelegate` (`|CreateDelegate` :!event `RecoverPlayer`) 10.0))
  (set `self.PlayerRecoverTimerHandler` _returnvalue_3))

(event `RecoverPlayer`
  ; Recover Player
  (`InGamePlayer.RecoverPlayerHP` (`self.InGamePlayer`)))

(event `SpawnMonster`
  (bind _randomlocation (`NavigationSystemV1.K2_GetRandomReachablePointInRadius` (`Actor.K2_GetActorLocation` (`self.InGamePlayer`)) 800.0 null null))
  ; Spawn Monster
  (if (< (`self.CurrentAliveCount`) (`self.MaxAliveCount`))
    (bind _returnvalue (`PoolManagerComponent.GetFromPool` (`self.PoolManagerRef`) (`KismetArrayLibrary.Array_Random` (`self.SpawnMonsterNames`))))
    (`/Engine/EditorBlueprintResources/StandardMacros.IsValid` _returnvalue
      (:`Is Valid`
        (`Actor.K2_SetActorLocation` _returnvalue (`KismetMathLibrary.MakeVector` (.x _randomlocation) (.y _randomlocation) 100.0) false true)
        (`Actor.K2_SetActorRotation` _returnvalue (`KismetMathLibrary.FindLookAtRotation` (`KismetMathLibrary.MakeVector` (.x _randomlocation) (.y _randomlocation) 100.0) (`Actor.K2_GetActorLocation` (`self.InGamePlayer`))) false)
        (`BaseMonster.EnableMonster` _returnvalue (`self.StatMultiplier`) (`self.LevelMultiplier`))
        (`KismetArrayLibrary.Array_AddUnique` (`self.CurrentMonsters`) _returnvalue)
        (`/Engine/EditorBlueprintResources/StandardMacros.IncrementInt` (`self.CurrentAliveCount`))))))

(event `EndWave`
  ; End Wave
  (`KismetSystemLibrary.K2_ClearAndInvalidateTimerHandle` (`self.SpawnMonsterTimeHandler`))
  (`KismetSystemLibrary.K2_ClearAndInvalidateTimerHandle` (`self.EndWaveTimeHandler`))
  (`self.ClearMonsters`)
  (`self.OnStageClear`))

(event `OnPlayerDie`
  ; Player Die
  (`KismetSystemLibrary.K2_ClearAndInvalidateTimerHandle` (`self.SpawnMonsterTimeHandler`))
  (`KismetSystemLibrary.K2_ClearAndInvalidateTimerHandle` (`self.EndWaveTimeHandler`))
  (`self.ClearMonsters`)
  (`self.OnStageFailed`))

(fn `ClearMonsters`
  (for _array_element (`self.CurrentMonsters`)
    (if (not (`Actor.bHidden` _array_element))
      (`BaseMonster.DisableMonster` _array_element)
      (`PoolManagerComponent.ReturnToPool` (`self.PoolManagerRef`) _array_element))))