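; Actor component that pools monsters for reuse, working with the game mode's wave manager.
; InitPool looks up each new name in DT_Monster, then pre-spawns disabled instances with table stats into a name-keyed map.
; GetFromPool returns the first hidden monster of that name, treating hidden state as availability.
; ReturntoPool stops movement and AI, disables visibility, collision and tick, and decrements the wave's alive count.
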(event `self.InitPool`
  (params (InNames :type "Array of Name (by ref)") (InSpawnCount :type Integer))
  ; Init Pool CPP
  (for _array_element InNames
    (if (not (`BlueprintMapLibrary.Map_Contains` (`self.MonsterPoolMap`) _array_element))
      (bind _returnvalue (`|GetDataTableRow` "/Game/Blueprints/Data/DataTable/DT_Monster.DT_Monster" _array_element)
        (:`then`
          (bind (_class _stat) (break `/Game/Blueprints/Data/Structure/S_Monster` _returnvalue))
          (`self.SpawnMonsters` _class _array_element _stat InSpawnCount))))))

(event `self.ReturnToPool`
  (params (InMonster :type "BaseMonster Object Reference"))
  ; Rethrn to Pool CPP
  (`MovementComponent.StopMovementImmediately` (`Character.CharacterMovement` InMonster))
  (`Actor.SetActorHiddenInGame` InMonster true)
  (`Actor.SetActorEnableCollision` InMonster false)
  (`Actor.SetActorTickEnabled` InMonster false)
  (`MonsterAIController.StopAI` (`BaseMonster.AIController` InMonster))
  (`WaveManagerComponent.DecreaseCurrentAliveCount` (`InGameMode.WaveManagerComp` (`self.InGameMode`))))

(fn `GetFromPool`
  (params (InName :type Name))
  (returns (Result :type "BaseMonster Object Reference"))
  (bind (_value _returnvalue) (`BlueprintMapLibrary.Map_Find` (`self.MonsterPoolMap`) InName))
  (if _returnvalue
    (for _array_element (`.PoolList` (break `MonsterPool` _value))
      (if (`Actor.bHidden` _array_element)
        (return _array_element)))
    (return null)
    (else
      (return null))))

(fn `SpawnMonsters`
  (params (InSpawnClass :type "/Game/Blueprints/Monster/BP_BaseMonster Class Reference") (InMonsterName :type Name) (InStat :type "/Game/Blueprints/Data/Structure/S_MonsterStat Structure") (InSpawnCount :type Integer))
  (locals (MonsterArray :type "Array of BaseMonster Object Reference"))
  (for _ (range 1 (+ InSpawnCount 1))
    (bind _returnvalue (`|SpawnActorFromClass` InSpawnClass (`KismetMathLibrary.MakeTransform` (0.0 0.0 0.0)) "AlwaysSpawn" "MultiplyWithRoot" null InStat null))
    (`/Game/Blueprints/Monster/BP_BaseMonster.DisabledMonster` _returnvalue)
    (`KismetArrayLibrary.Array_Add` (`local.MonsterArray`) _returnvalue))
  (`BlueprintMapLibrary.Map_Add` (`self.MonsterPoolMap`) InMonsterName (make `MonsterPool` (`local.MonsterArray`))))