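; Wave manager component that runs one timed stage of monster spawning around the player.
; Init reads the stage's DTWave row and fills the monster pool; StartGame starts looping spawn and wave-end timers.
; Spawns activate random pooled monsters near the player with a stat multiplier, up to a count cap.
; Wave end returns visible monsters and signals stage clear; GoNextStage saves player progress to the GameInstance and opens InventoryMap.
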(event `self.ReceiveBeginPlay`
  (`self.SetPlayer`))

(event `Init`
  (params (InStage :type Integer) (InPoolManagerRef :type "/Game/Blueprints/Wave/BP_PoolManagerComponent Object Reference"))
  ; Initialize
  (set `self.PoolManagerRef` InPoolManagerRef)
  (set `self.CurrentStage` InStage)
  (bind _returnvalue (`|GetDataTableRow` (`self.DT_Wave`) (`KismetStringLibrary.Conv_StringToName` (`KismetStringLibrary.Conv_IntToString` (`self.CurrentStage`))))
    (:`then`
      (bind (_stagenum _spawnmonsters _spawncount _time _spawninterval _statmultiplier) (break `/Game/Blueprints/Data/Structure/S_Wave` _returnvalue))
      (set `self.SpawnMonsterNames` _spawnmonsters)
      (set `self.SpawnInterval` _spawninterval)
      (set `self.StatMultiplier` _statmultiplier)
      (set `self.MaxAliveCount` _spawncount)
      (set `self.WaveTimer` _time)
      (`/Game/Blueprints/Wave/BP_PoolManagerComponent.InitPool` (`self.PoolManagerRef`) (`self.SpawnMonsterNames`) (`self.MaxAliveCount`)))))

(event `StartGame`
  ; StartGame
  (bind _returnvalue (`KismetSystemLibrary.K2_SetTimerDelegate` (`|CreateDelegate` :!event `SpawnMonster`) (`self.SpawnInterval`) true))
  (set `self.SpawnMonsterTimeHandler` _returnvalue)
  (bind _returnvalue_2 (`KismetSystemLibrary.K2_SetTimerDelegate` (`|CreateDelegate` :!event `EndWave`) (`self.WaveTimer`)))
  (set `self.EndWaveTimeHandler` _returnvalue_2)
  (set `self.CurrentAliveCount` 0))

(event `SpawnMonster`
  (bind _randomlocation (`NavigationSystemV1.K2_GetRandomReachablePointInRadius` (`Actor.K2_GetActorLocation` (`self.BP_Player`)) 1500.0 null null))
  ; Spawn Monster
  (if (< (`self.CurrentAliveCount`) (`self.MaxAliveCount`))
    (bind _result (`/Game/Blueprints/Wave/BP_PoolManagerComponent.GetFromPool` (`self.PoolManagerRef`) (`KismetArrayLibrary.Array_Random` (`self.SpawnMonsterNames`))))
    (`/Engine/EditorBlueprintResources/StandardMacros.IsValid` _result
      (:`Is Valid`
        (`Actor.K2_SetActorLocation` _result (`KismetMathLibrary.MakeVector` (.x _randomlocation) (.y _randomlocation) 100.0) false true)
        (`/Game/Blueprints/Monster/BP_BaseMonster.ActiveMonster` _result (`self.StatMultiplier`))
        (`KismetArrayLibrary.Array_AddUnique` (`self.CurrentMonsters`) _result)
        (`/Engine/EditorBlueprintResources/StandardMacros.IncrementInt` (`self.CurrentAliveCount`))))))

(event `EndWave`
  ; End Wave
  (`KismetSystemLibrary.K2_ClearAndInvalidateTimerHandle` (`self.SpawnMonsterTimeHandler`))
  (`KismetSystemLibrary.K2_ClearAndInvalidateTimerHandle` (`self.EndWaveTimeHandler`))
  (`self.ClearMonsters`)
  (`self.OnStageClear`))

(fn `ClearMonsters`
  (for _array_element (`self.CurrentMonsters`)
    (if (not (`Actor.bHidden` _array_element))
      (`/Game/Blueprints/Monster/BP_BaseMonster.DisabledMonster` _array_element)
      (`/Game/Blueprints/Wave/BP_PoolManagerComponent.ReturnToPool` (`self.PoolManagerRef`) _array_element))))

(fn `GoNextStage`
  (bind _bp_player (`self.BP_Player`))
  (bind _asbp_god_of_weapon_game_instance (cast `/Game/Blueprints/BP_GodOfWeaponGameInstance` (`GameplayStatics.GetGameInstance`)))
  (`/Engine/EditorBlueprintResources/StandardMacros.IsValid` _asbp_god_of_weapon_game_instance
    (:`Is Valid`
      (set `GodOfWeaponGameInstance.PlayerStat` (`/Game/Blueprints/Player/BP_Player.PlayerStat` _bp_player) _asbp_god_of_weapon_game_instance)
      (set `GodOfWeaponGameInstance.PlayerCoin` (`/Game/Blueprints/Player/BP_Player.CoinCnt` _bp_player) _asbp_god_of_weapon_game_instance)
      (`/Engine/EditorBlueprintResources/StandardMacros.IncrementInt` (`/Game/Blueprints/BP_GodOfWeaponGameInstance.CurrentStage` _asbp_god_of_weapon_game_instance)
        (:`  `
          (`GameplayStatics.OpenLevelBySoftObjectPtr` "/Game/Maps/InventoryMap.InventoryMap"))))))

(fn `SetPlayer`
  (bind _asbp_player (cast `/Game/Blueprints/Player/BP_Player` (`GameplayStatics.GetPlayerPawn` 0)))
  (`/Engine/EditorBlueprintResources/StandardMacros.IsValid` _asbp_player
    (:`Is Valid`
      (set `self.BP_Player` _asbp_player))))