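; Monster pool manager component that pre-spawns and recycles monsters for the wave system.
; InitPool looks up each new name in the monster DataTable, spawns disabled copies with their stats, and stores them per name in a map.
; GetFromPool returns the first hidden monster of that name, or nothing when none is free.
; ReturnToPool stops, hides and disables the monster, then decrements the wave manager's alive count through the game mode.
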(event `self.ReceiveBeginPlay`
  (bind _asgm_in_game (cast `/Game/Blueprints/GameMode/GM_InGame` (`GameplayStatics.GetGameMode`)))
  (`/Engine/EditorBlueprintResources/StandardMacros.IsValid` _asgm_in_game
    (:`Is Valid`
      (set `self.GM_InGame` _asgm_in_game))))

(event `InitPool`
  (params (InNames :type "Array of Name") (InSpawnCount :type Integer :default 50))
  (for _array_element InNames
    (if (not (`BlueprintMapLibrary.Map_Contains` (`self.MonsterPoolMap`) _array_element))
      (bind _returnvalue (`|GetDataTableRow` (`self.DT_Monster`) _array_element)
        (:`then`
          (bind (_class _stat) (break `/Game/Blueprints/Data/Structure/S_Monster` _returnvalue))
          (`self.SpawnMonsters` _class _array_element _stat InSpawnCount))))))

(fn `GetFromPool`
  (params (InName :type Name))
  (returns (Result :type "/Game/Blueprints/Monster/BP_BaseMonster Object Reference"))
  (bind (_value _returnvalue) (`BlueprintMapLibrary.Map_Find` (`self.MonsterPoolMap`) InName))
  (if _returnvalue
    (for _array_element (`.PoolList_4_434BA7C2438284F433C62983461A60CC` (break `/Game/Blueprints/Data/Structure/S_MonsterPool` _value))
      (if (`Actor.bHidden` _array_element)
        (return _array_element)))
    (return null)
    (else
      (return null))))

(fn `ReturnToPool`
  (params (InMonster :type "/Game/Blueprints/Monster/BP_BaseMonster Object Reference"))
  (`MovementComponent.StopMovementImmediately` (`Character.CharacterMovement` InMonster))
  (`Actor.SetActorHiddenInGame` InMonster true)
  (`Actor.SetActorEnableCollision` InMonster false)
  (`Actor.SetActorTickEnabled` InMonster false)
  (`/Engine/EditorBlueprintResources/StandardMacros.DecrementInt` (`/Game/Blueprints/Wave/BP_WaveManagerComponent.CurrentAliveCount` (`/Game/Blueprints/GameMode/GM_InGame.BP_WaveManagerComponent` (`self.GM_InGame`)))))

(fn `SpawnMonsters`
  (params (InSpawnClass :type "/Game/Blueprints/Monster/BP_BaseMonster Class Reference") (InMonsterName :type Name) (InStat :type "/Game/Blueprints/Data/Structure/S_MonsterStat Structure") (InSpawnCount :type Integer))
  (locals (MonsterArray :type "Array of /Game/Blueprints/Monster/BP_BaseMonster Object Reference"))
  (for _ (range 1 (+ InSpawnCount 1))
    (bind _returnvalue (`|SpawnActorFromClass` InSpawnClass (`KismetMathLibrary.MakeTransform` (0.0 0.0 0.0)) "Undefined" "MultiplyWithRoot" null InStat null))
    (`/Game/Blueprints/Monster/BP_BaseMonster.DisabledMonster` _returnvalue)
    (`KismetArrayLibrary.Array_Add` (`local.MonsterArray`) _returnvalue))
  (`BlueprintMapLibrary.Map_Add` (`self.MonsterPoolMap`) InMonsterName (make `/Game/Blueprints/Data/Structure/S_MonsterPool` (`local.MonsterArray`))))