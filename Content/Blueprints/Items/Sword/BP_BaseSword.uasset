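; Base sword item that performs a sequence-driven attack and damages monsters it touches.
; Attack turns off the owner spring arm's pawn control rotation and plays the attack Actor Sequence.
; The finish event, also called after a short delay if the item state still matches, changes state and calls Returning.
; Attack box overlaps apply the item's stat damage to Monster-tagged actors, crediting the first player controller.
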(event `self.Attack`
  (set `SpringArmComponent.bUsePawnControlRotation` false (`self.OwnerSpringArm`))
  (`ActorSequenceComponent.PlaySequence` (`self.AttackActorSequence`))
  (`KismetSystemLibrary.Delay` 0.5)
  (if (`|EnumEquality` (`self.ItemCurrentState`) "NewEnumerator2")
    (`self.OnFinishAttackSequence`)))

(event `self.AttackBoxCollision.OnComponentBeginOverlap`
  (params (OverlappedComponent :type "PrimitiveComponent Object Reference") (OtherActor :type "Actor Object Reference") (OtherComp :type "PrimitiveComponent Object Reference") (OtherBodyIndex :type Integer) (bFromSweep :type Boolean) (SweepResult :type "HitResult Structure (by ref)"))
  (bind _itemstat_damage (break `ItemStatStructure` (`self.ItemStat`)))
  (if (`self.ActorHasTag` OtherActor "Monster")
    (`GameplayStatics.ApplyDamage` OtherActor _itemstat_damage (`GameplayStatics.GetPlayerController` 0) self "/Script/Engine.DamageType")))

(event `OnFinishAttackSequence`
  (set `self.ItemCurrentState` "NewEnumerator3")
  (`self.Returning`))

(fn `UserConstructionScript`
  (`parent.UserConstructionScript`))