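; Base actor for a player's attack item, which leaves its spring arm to strike the nearest monster within range, then returns.
; An Idle, Approach, Attacking, Returning, Cooldown state machine polls a range sphere on Tick while idle.
; Timelines lerp movement at constant height, detaching and reattaching the owning child actor component.
; Attack is a delay-only placeholder for child overrides, and Init scales item stats by player multipliers.
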(event `self.ReceiveBeginPlay`
  (`self.SetPlayer`))

(event `self.ReceiveTick`
  (params (DeltaSeconds :type "Float (single-precision)"))
  (switch `/Game/Blueprints/Data/Enum/E_AttackItemState` (`self.ItemCurrentState`)
    (:`NewEnumerator0`
      (`self.Idle`))))

(event `Idle`
  ; Idle Events : False일 경우 Idle Animation!
  (if (and (`self.IsCanAttack?`) (`self.IsMonsterInRange?`))
    (set `self.ItemCurrentState` "NewEnumerator1")
    (set `self.bCanAttack` false)
    (`self.Approch`)))

(event `MoveToTarget`
  (params (InStartLocation :type "Vector Structure") (InTargetLocation :type "Vector Structure"))
  ; Approch
  (`SceneComponent.K2_DetachFromComponent` (`self.OwnerChildActorComponent`) "KeepWorld" "KeepWorld" "KeepWorld" true)
  (bind (_direction _alpha) (`Timeline|TL_MoveToMonster`)
    (:`Update`
      (`self.K2_SetActorLocation` (`KismetMathLibrary.VLerp` (`KismetMathLibrary.MakeVector` InStartLocation_X InStartLocation_Y InStartLocation_Z) (`KismetMathLibrary.MakeVector` InTargetLocation_X InTargetLocation_Y InStartLocation_Z) _alpha)))
    (:`Finished`
      (set `self.ItemCurrentState` "NewEnumerator2")
      (`self.Attack`))))

(event `Approch`
  ; Approch
  (bind (_targetactor _targetlocation) (`self.FindTargetInRange`))
  (`/Engine/EditorBlueprintResources/StandardMacros.IsValid` _targetactor
    (:`Is Valid`
      (`self.MoveToTarget` (`self.K2_GetActorLocation`) _targetlocation))))

(event `Attack`
  ; Attack - Override 해야 함
  (`KismetSystemLibrary.Delay` 0.2)
  (set `self.ItemCurrentState` "NewEnumerator3")
  (`self.Returning`))

(event `Returning`
  (bind _ownerspringarm (`self.OwnerSpringArm`))
  ; Returning
  (set `SpringArmComponent.bUsePawnControlRotation` true _ownerspringarm)
  (`self.ReturnToTarget` (`self.K2_GetActorLocation`) (`SceneComponent.GetSocketLocation` _ownerspringarm (`SceneComponent.GetAttachSocketName` _ownerspringarm))))

(event `ReturnToTarget`
  (params (InStartLocation :type "Vector Structure") (InTargetLocation :type "Vector Structure"))
  ; Returning
  (bind (_direction _alpha) (`Timeline|TL_MoveToReturn`)
    (:`Update`
      (`self.K2_SetActorLocation` (`KismetMathLibrary.VLerp` (`KismetMathLibrary.MakeVector` InStartLocation_X InStartLocation_Y InStartLocation_Z) (`KismetMathLibrary.MakeVector` InTargetLocation_X InTargetLocation_Y InStartLocation_Z) _alpha)))
    (:`Finished`
      ;; Re Attach
      (`SceneComponent.K2_AttachToComponent` (`self.OwnerChildActorComponent`) (`self.OwnerSpringArm`) "None" "KeepWorld" "KeepWorld" "KeepWorld" true)
      (set `self.ItemCurrentState` "NewEnumerator4")
      (`self.Cooldown`))))

(event `Cooldown`
  (bind (_itemstat_damage _itemstat_attackrange _itemstat_attackspeed _itemstat_cooldowntime) (break `ItemStatStructure` (`self.ItemStat`)))
  ; Cool Down
  (`KismetSystemLibrary.K2_SetTimerDelegate` (`|CreateDelegate` :!event `OnCooldownFinished`) (/ _itemstat_cooldowntime _itemstat_attackspeed)))

(event `OnCooldownFinished`
  ; Cool Down
  (set `self.bCanAttack` true)
  (set `self.ItemCurrentState` "NewEnumerator0"))

(fn `FindTargetInRange`
  (returns (TargetActor :type "Actor Object Reference") (TargetLocation :type "Vector Structure"))
  (locals (NearetTargetRef :type "Actor Object Reference") (NearetLength :type "Float (double-precision)" :default 0.0))
  (set `local.NearetTargetRef` null)
  (for (_array_element _array_index) (`PrimitiveComponent.GetOverlappingActors` (`self.RangeSphereCollision`) "/Game/Blueprints/Monster/BP_BaseMonster.BP_BaseMonster_C")
    (if (== _array_index 0)
      ; First로 초기화
      (set `local.NearetTargetRef` _array_element)
      (bind _distance (`/Game/Blueprints/Utils/BPFL_Utils.GetDistance` (`self.K2_GetActorLocation` (`local.NearetTargetRef`)) (`self.K2_GetActorLocation`)))
      (set `local.NearetLength` _distance)
      (else
        ; Nearest Update
        (bind _distance_2 (`/Game/Blueprints/Utils/BPFL_Utils.GetDistance` (`self.K2_GetActorLocation` _array_element) (`self.K2_GetActorLocation`)))
        (if (< _distance_2 (`local.NearetLength`))
          (set `local.NearetTargetRef` _array_element)
          (set `local.NearetLength` _distance_2)))))
  ; Return
  (return (`local.NearetTargetRef`) (`self.K2_GetActorLocation` (`local.NearetTargetRef`))))

(fn `Init`
  (params (InItemTypes :type "EItemType Enum" :default "Sword") (InItemStat :type "ItemStatStructure Structure") (InOwnerSpringArm :type "SpringArmComponent Object Reference") (InOwnerChildActorComponent :type "ChildActorComponent Object Reference"))
  (bind _bp_player (`self.BP_Player`))
  (bind (_itemstat_damage _itemstat_attackrange) (break `ItemStatStructure` (`self.ItemStat`)))
  (bind (_playerstat_currenthp _playerstat_maxhp _playerstat_shortrangeattackforce _playerstat_longrangeattackforce _playerstat_attackspeedmultifier _playerstat_movespeedmultifier _playerstat_attackrangemultifier) (break `PlayerStatStructure` (`/Game/Blueprints/Player/BP_Player.PlayerStat` _bp_player)))
  (set `self.ItemType` InItemTypes)
  (set `self.OwnerSpringArm` InOwnerSpringArm)
  (set `self.OwnerChildActorComponent` InOwnerChildActorComponent)
  (`/Engine/EditorBlueprintResources/StandardMacros.IsValid` _bp_player
    (:`Is Valid`
      (set `self.ItemStat` (make `ItemStatStructure` (* InItemStat_Damage _playerstat_shortrangeattackforce) (* InItemStat_AttackRange _playerstat_attackrangemultifier) (* InItemStat_AttackSpeed _playerstat_attackspeedmultifier) InItemStat_CooldownTime))
      (`SphereComponent.SetSphereRadius` (`self.RangeSphereCollision`) _itemstat_attackrange true))))

(fn `IsCanAttack?`
  (returns (Result :type Boolean))
  (return (and (`|EnumEquality` (`self.ItemCurrentState`) "NewEnumerator0") (`self.bCanAttack`))))

(fn `IsMonsterInRange?`
  (returns (Result :type Boolean))
  (return (> (`KismetArrayLibrary.Array_Length` (`PrimitiveComponent.GetOverlappingActors` (`self.RangeSphereCollision`) "/Game/Blueprints/Monster/BP_BaseMonster.BP_BaseMonster_C")) 0)))

(fn `SetPlayer`
  (bind _asbp_player (cast `/Game/Blueprints/Player/BP_Player` (`GameplayStatics.GetPlayerPawn` 0)))
  (`/Engine/EditorBlueprintResources/StandardMacros.IsValid` _asbp_player
    (:`Is Valid`
      (set `self.BP_Player` _asbp_player))))

(fn `UserConstructionScript`)