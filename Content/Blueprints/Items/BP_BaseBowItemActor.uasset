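; Base bow item actor that automatically shoots arrows at the nearest monster within its range sphere.
; An Idle, Attacking and Cooldown state machine polls for targets on Tick, turns toward the closest, spawns a BP_PlayerArrow, then waits on a timer scaled by attack speed.
; Init scales damage, range and attack speed by the player's stats and resizes the sphere to match.
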(event `self.ReceiveBeginPlay`
  (`self.SetPlayer`))

(event `self.ReceiveTick`
  (params (DeltaSeconds :type "Float (single-precision)"))
  (switch `/Game/Blueprints/Data/Enum/E_BowItemState` (`self.ItemCurrentState`)
    (:`NewEnumerator0`
      (`self.Idle`))))

(event `Idle`
  ; Idle Events : False일 경우 Idle Animation!
  (if (and (`self.IsCanAttack?`) (`self.InMonsterInRange?`))
    (set `self.ItemCurrentState` "NewEnumerator2")
    (set `self.bCanAttack` false)
    (`self.Attacking`)))

(event `Attacking`
  (bind _returnvalue (`self.K2_GetActorLocation`))
  (bind _itemstat_damage (break `ItemStatStructure` (`self.ItemStat`)))
  ; Spawn Bow
  (bind (_targetactor _targetlocation) (`self.FindTargetInRange`))
  (`/Engine/EditorBlueprintResources/StandardMacros.IsValid` _targetactor
    (:`Is Valid`
      (bind _returnvalue_2 (`KismetMathLibrary.FindLookAtRotation` _returnvalue _targetlocation))
      (`self.K2_SetActorRotation` _returnvalue_2)
      (`|SpawnActorFromClass` "/Game/Blueprints/Items/BP_PlayerArrow.BP_PlayerArrow_C" (`KismetMathLibrary.MakeTransform` _returnvalue _returnvalue_2) "Undefined" "MultiplyWithRoot" null (`self.ArrowStaticMesh`) (`self.ArrowNiagara`) _itemstat_damage null)
      (set `self.ItemCurrentState` "NewEnumerator4")
      (`self.Cooldown`))))

(event `Cooldown`
  (bind (_itemstat_damage _itemstat_attackrange _itemstat_attackspeed _itemstat_cooldowntime) (break `ItemStatStructure` (`self.ItemStat`)))
  ; Cooldown
  (`KismetSystemLibrary.K2_SetTimerDelegate` (`|CreateDelegate` :!event `OnCooldownFinished`) (/ _itemstat_cooldowntime _itemstat_attackspeed)))

(event `OnCooldownFinished`
  ; Cooldown
  (set `self.bCanAttack` true)
  (set `self.ItemCurrentState` "NewEnumerator0"))

(fn `FindTargetInRange`
  (returns (TargetActor :type "Actor Object Reference") (TargetLocation :type "Vector Structure"))
  (locals (NearetTargetRef :type "Actor Object Reference") (NearetLength :type "Float (double-precision)"))
  (set `local.NearetTargetRef` null)
  (for (_array_element _array_index) (`PrimitiveComponent.GetOverlappingActors` (`self.RangeSphereCollision`) "/Game/Blueprints/Monster/BP_BaseMonster.BP_BaseMonster_C")
    (if (== _array_index 0)
      ; First로 초기화
      (set `local.NearetTargetRef` _array_element)
      (bind _distance (`/Game/Blueprints/Utils/BPFL_Utils.GetDistance` (`self.K2_GetActorLocation` (`local.NearetTargetRef`)) (`self.K2_GetActorLocation`)))
      (set `local.NearetLength` _distance)
      (else
        ; Nearest Update
        (bind _distance_2 (`/Game/Blueprints/Utils/BPFL_Utils.GetDistance` (`self.K2_GetActorLocation` _array_element) (`self.K2_GetActorLocation`)))
        (if (< _distance_2 (`local.NearetLength`))
          (set `local.NearetTargetRef` _array_element)
          (set `local.NearetLength` _distance_2)))))
  ; Return
  (return (`local.NearetTargetRef`) (`self.K2_GetActorLocation` (`local.NearetTargetRef`))))

(fn `Init`
  (params (InItemType :type "EItemType Enum" :default "Sword") (InItemStat :type "ItemStatStructure Structure"))
  (bind _bp_player (`self.BP_Player`))
  (bind (_playerstat_currenthp _playerstat_maxhp _playerstat_shortrangeattackforce _playerstat_longrangeattackforce _playerstat_attackspeedmultifier _playerstat_movespeedmultifier _playerstat_attackrangemultifier) (break `PlayerStatStructure` (`/Game/Blueprints/Player/BP_Player.PlayerStat` _bp_player)))
  (bind _returnvalue (* InItemStat_AttackRange _playerstat_attackrangemultifier))
  (set `self.ItemType` InItemType)
  (`/Engine/EditorBlueprintResources/StandardMacros.IsValid` _bp_player
    (:`Is Valid`
      (set `self.ItemStat` (make `ItemStatStructure` (* InItemStat_Damage _playerstat_longrangeattackforce) _returnvalue (* InItemStat_AttackSpeed _playerstat_attackspeedmultifier) InItemStat_CooldownTime))
      (`SphereComponent.SetSphereRadius` (`self.RangeSphereCollision`) _returnvalue true))))

(fn `InMonsterInRange?`
  (returns (Result :type Boolean))
  (return (> (`KismetArrayLibrary.Array_Length` (`PrimitiveComponent.GetOverlappingActors` (`self.RangeSphereCollision`) "/Game/Blueprints/Monster/BP_BaseMonster.BP_BaseMonster_C")) 0)))

(fn `IsCanAttack?`
  (returns (Result :type Boolean))
  (return (and (`|EnumEquality` (`self.ItemCurrentState`) "NewEnumerator0") (`self.bCanAttack`))))

(fn `SetPlayer`
  (bind _asbp_player (cast `/Game/Blueprints/Player/BP_Player` (`GameplayStatics.GetPlayerPawn` 0)))
  (`/Engine/EditorBlueprintResources/StandardMacros.IsValid` _asbp_player
    (:`Is Valid`
      (set `self.BP_Player` _asbp_player))))

(fn `UserConstructionScript`)