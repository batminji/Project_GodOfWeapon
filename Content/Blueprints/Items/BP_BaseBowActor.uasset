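; Base bow item actor that automatically shoots arrows at monsters in range.
; An Idle, Attacking, Cooldown state cycle gates firing: when attack is allowed, it turns toward the found target and spawns a BP_PlayerArrow toward it.
; The arrow receives the bow's mesh, Niagara effect and damage stat.
; A timer set to cooldown time divided by attack speed governs the delay between shots.
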(event `self.Idle`
  ; Idle Events : False일 경우 Idle Animation!
  (if (and (`self.IsCanAttack`) (`self.IsMonsterInRange`))
    (set `self.ItemCurrentState` "Attacking")
    (set `self.bCanAttack` false)
    (`self.Attack`)))

(event `self.Attack`
  (bind _returnvalue (`self.K2_GetActorLocation`))
  (bind _itemstat_damage (break `ItemStat` (`self.ItemStat`)))
  ; Spawn Bow
  (bind (_outtargetactor _outtargetlocation) (`self.FindTargetInRange`))
  (`/Engine/EditorBlueprintResources/StandardMacros.IsValid` _outtargetactor
    (:`Is Valid`
      (bind _returnvalue_2 (`KismetMathLibrary.FindLookAtRotation` _returnvalue _outtargetlocation))
      (`self.K2_SetActorRotation` _returnvalue_2)
      (`|SpawnActorFromClass` "/Game/Blueprints/Items/BP_PlayerArrow.BP_PlayerArrow_C" (`KismetMathLibrary.MakeTransform` _returnvalue _returnvalue_2) "Undefined" "MultiplyWithRoot" null (`self.ArrowStaticMesh`) (`self.ArrowNiagaraSystem`) _itemstat_damage null)
      (set `self.ItemCurrentState` "Cooldown")
      (`self.Cooldown`))))

(event `self.Cooldown`
  (bind (_itemstat_damage _itemstat_attackrange _itemstat_attackspeed _itemstat_cooldowntime) (break `ItemStat` (`self.ItemStat`)))
  ; Cooldown
  (`KismetSystemLibrary.K2_SetTimerDelegate` (`|CreateDelegate` :!event `OnCooldownFinished`) (/ _itemstat_cooldowntime _itemstat_attackspeed)))

(event `self.OnCooldownFinished`
  ; Cooldown
  (set `self.bCanAttack` true)
  (set `self.ItemCurrentState` "Idle"))

(fn `UserConstructionScript`
  (`parent.UserConstructionScript`))