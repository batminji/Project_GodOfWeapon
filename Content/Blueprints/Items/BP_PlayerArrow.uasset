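; BP_PlayerArrow is the player's arrow actor, which damages monsters it hits.
; On BeginPlay it runs the parent logic, then applies the supplied static mesh and Niagara system to its components.
; When its box component overlaps an actor tagged "Monster", it applies AttackDamage with player controller 0 as instigator, then destroys itself.
; Overlaps with untagged actors are ignored, and no movement logic appears in these graphs.
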(event `self.ReceiveBeginPlay`
  (`parent.ReceiveBeginPlay`)
  (`StaticMeshComponent.SetStaticMesh` (`self.ArrowMeshComponent`) (`self.InStaticMesh`))
  (`NiagaraComponent.SetAsset` (`self.NiagaraComponent`) (`self.InNiagaraSystemAsset`) true))

(event `self.BoxComponent.OnComponentBeginOverlap`
  (params (OverlappedComponent :type "PrimitiveComponent Object Reference") (OtherActor :type "Actor Object Reference") (OtherComp :type "PrimitiveComponent Object Reference") (OtherBodyIndex :type Integer) (bFromSweep :type Boolean) (SweepResult :type "HitResult Structure (by ref)"))
  (if (`self.ActorHasTag` OtherActor "Monster")
    (`GameplayStatics.ApplyDamage` OtherActor (`self.AttackDamage`) (`GameplayStatics.GetPlayerController` 0) self "/Script/Engine.DamageType")
    (`self.K2_DestroyActor`)))

(fn `UserConstructionScript`)