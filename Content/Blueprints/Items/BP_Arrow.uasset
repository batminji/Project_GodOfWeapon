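; BP_Arrow is an arrow projectile actor that damages monsters on contact.
; On BeginPlay it sets a five-second lifespan and assigns its static mesh and Niagara effect from input variables, so one class serves different arrow looks.
; When its Box collider overlaps an actor tagged Monster, it applies AttackDamage credited to the first player controller and destroys itself.
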(event `self.ReceiveBeginPlay`
  (`self.SetLifeSpan` 5.0)
  (`StaticMeshComponent.SetStaticMesh` (`self.ArrowStaticMesh`) (`self.InStaticMesh`))
  (`NiagaraComponent.SetAsset` (`self.Niagara`) (`self.InNiagaraSystemAsset`) true))

(event `self.Box.OnComponentBeginOverlap`
  (params (OverlappedComponent :type "PrimitiveComponent Object Reference") (OtherActor :type "Actor Object Reference") (OtherComp :type "PrimitiveComponent Object Reference") (OtherBodyIndex :type Integer) (bFromSweep :type Boolean) (SweepResult :type "HitResult Structure (by ref)"))
  (if (`self.ActorHasTag` OtherActor "Monster")
    (`GameplayStatics.ApplyDamage` null (`self.AttackDamage`) (`GameplayStatics.GetPlayerController` 0) self "/Script/Engine.DamageType")
    (`self.K2_DestroyActor`)))

(fn `UserConstructionScript`)