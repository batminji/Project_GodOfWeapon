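; Base attack item actor that rides on an owner's spring arm and launches itself at monsters in range.
; An enum-style state cycle runs Idle, Approach, Attacking, Returning and Cooldown through chained events, with Attack as a placeholder for override.
; It detaches its child actor component, moves out and back with timeline lerps at fixed height, then reattaches.
; A timer scaled by cooldown time and attack speed gates the next attack.
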(event `self.Idle`
  ; Idle Events : False일 경우 Idle Animation!
  (if (and (`self.IsCanAttack`) (`self.IsMonsterInRange`))
    (set `self.ItemCurrentState` "Approach")
    (set `self.bCanAttack` false)
    (`self.Approach`)))

(event `MoveToTarget`
  (params (InStartLocation :type "Vector Structure") (InTargetLocation :type "Vector Structure"))
  ; Approch
  (`SceneComponent.K2_DetachFromComponent` (`self.OwnerChildActor`) "KeepWorld" "KeepWorld" "KeepWorld" true)
  (bind (_direction _alpha) (`Timeline|TL_MoveToMonster`)
    (:`Update`
      (`self.K2_SetActorLocation` (`KismetMathLibrary.VLerp` (`KismetMathLibrary.MakeVector` InStartLocation_X InStartLocation_Y InStartLocation_Z) (`KismetMathLibrary.MakeVector` InTargetLocation_X InTargetLocation_Y InStartLocation_Z) _alpha)))
    (:`Finished`
      (set `self.ItemCurrentState` "Attacking")
      (`self.Attack`))))

(event `self.Approach`
  ; Approch
  (bind (_outtargetactor _outtargetlocation) (`self.FindTargetInRange`))
  (`/Engine/EditorBlueprintResources/StandardMacros.IsValid` _outtargetactor
    (:`Is Valid`
      (`self.MoveToTarget` (`self.K2_GetActorLocation`) _outtargetlocation))))

(event `self.Attack`
  ; Attack - Override 해야 함
  (`KismetSystemLibrary.Delay` 0.2)
  (set `self.ItemCurrentState` "Returning")
  (`self.Returning`))

(event `self.Returning`
  (bind _ownerspringarm (`self.OwnerSpringArm`))
  ; Returning
  (set `SpringArmComponent.bUsePawnControlRotation` true _ownerspringarm)
  (`self.ReturnToTarget` (`self.K2_GetActorLocation`) (`SceneComponent.GetSocketLocation` _ownerspringarm (`SceneComponent.GetAttachSocketName` _ownerspringarm))))

(event `ReturnToTarget`
  (params (InStartLocation :type "Vector Structure") (InTargetLocation :type "Vector Structure"))
  ; Returning
  (bind (_direction _alpha) (`Timeline|TL_MoveToReturn`)
    (:`Update`
      (`self.K2_SetActorLocation` (`KismetMathLibrary.VLerp` (`KismetMathLibrary.MakeVector` InStartLocation_X InStartLocation_Y InStartLocation_Z) (`KismetMathLibrary.MakeVector` InTargetLocation_X InTargetLocation_Y InStartLocation_Z) _alpha)))
    (:`Finished`
      ;; Re Attach
      (`SceneComponent.K2_AttachToComponent` (`self.OwnerChildActor`) (`self.OwnerSpringArm`) "None" "KeepWorld" "KeepWorld" "KeepWorld" true)
      (set `self.ItemCurrentState` "Cooldown")
      (`self.Cooldown`))))

(event `self.Cooldown`
  (bind (_itemstat_damage _itemstat_attackrange _itemstat_attackspeed _itemstat_cooldowntime) (break `ItemStat` (`self.ItemStat`)))
  ; Cool Down
  (`KismetSystemLibrary.K2_SetTimerDelegate` (`|CreateDelegate` :!event `OnCooldownFinished`) (/ _itemstat_cooldowntime _itemstat_attackspeed)))

(event `self.OnCooldownFinished`
  ; Cool Down
  (set `self.bCanAttack` true)
  (set `self.ItemCurrentState` "Idle"))

(fn `UserConstructionScript`
  (`parent.UserConstructionScript`))