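; BP_BaseMonster is the base monster Blueprint, adding damage filtering, attack playback and visual feedback on top of its parent class's logic.
; Damage applies only from causers tagged PlayerAttack, and the attack montage signals attack finish whether completed or interrupted.
; Enabling passes stat and level multipliers to the parent, then spawns Niagara at a downward trace hit.
; Separate events spawn coins and show floating damage widgets at the monster's projected screen position.
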(event `self.ReceiveAnyDamage`
  (params (Damage :type "Float (single-precision)") (DamageType :type "DamageType Object Reference") (InstigatedBy :type "Controller Object Reference") (DamageCauser :type "Actor Object Reference"))
  ; Damage Event
  (if (`self.ActorHasTag` DamageCauser "PlayerAttack")
    (`self.ApplyMonsterDamage` Damage)))

(event `self.EnableMonster`
  (params (InStatMultiplier :type "Float (single-precision)") (InLevelMultiplier :type "Float (single-precision)"))
  (bind _returnvalue (`self.K2_GetActorLocation`))
  ; Enable Monster
  (`parent.EnableMonster` InStatMultiplier InLevelMultiplier)
  (bind _outhit (`KismetSystemLibrary.LineTraceSingleForObjects` _returnvalue (- _returnvalue (0.0 0.0 1000.0)) (`|MakeArray` "ObjectTypeQuery9" :!type "EObjectTypeQuery Enum")))
  (`NiagaraFunctionLibrary.SpawnSystemAtLocation` (`self.SpawnNiagara`) (`.Location` (`GameplayStatics.BreakHitResult` _outhit)) (struct) (2.0 2.0 2.0)))

(event `Attack`
  ; Attack Montage
  (`|PlayMontage` (`self.Mesh`) (`self.AttackMontage`) 1.0 0.0 "Attack"
    (:`OnCompleted`
      _)
    (:`OnInterrupted`
      _))
  (`self.OnFinishAttack`))

(event `self.CreateCoinActors`
  (params (InCount :type Integer))
  ; Create Coin
  (for _ (range 1 (+ InCount 1))
    (`|SpawnActorFromClass` "/Game/Blueprints/Items/Coin/BP_Coin.BP_Coin_C" (`KismetMathLibrary.MakeTransform` (`self.K2_GetActorLocation`)) "Undefined" "MultiplyWithRoot" null null)))

(event `self.CreateDamageTextWidget`
  (params (InDamage :type Integer))
  ; Damage Text
  (bind _returnvalue (`|CreateWidget` "/Game/UI/InGame/WBP_FloatingDamage.WBP_FloatingDamage_C" null InDamage))
  (`UserWidget.AddToViewport` _returnvalue 0)
  (`UserWidget.SetPositionInViewport` _returnvalue (`WidgetLayoutLibrary.ProjectWorldLocationToWidgetPosition` (`GameplayStatics.GetPlayerController` 0) (`self.K2_GetActorLocation`) true) false))

(fn `UserConstructionScript`)