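; BP_Slime is a slime monster that deals melee damage to actors tagged Player through an attack collision component.
; OnStartAttack enables AttackCollision and clears the HitActors list, and OnEndAttack disables the collision.
; On overlap, it applies the current monster stat's base damage with AICMonster as instigator, recording each target in HitActors so it is hit only once per attack.
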(event `self.AttackCollision.OnComponentBeginOverlap`
  (params (OverlappedComponent :type "PrimitiveComponent Object Reference") (OtherActor :type "Actor Object Reference") (OtherComp :type "PrimitiveComponent Object Reference") (OtherBodyIndex :type Integer) (bFromSweep :type Boolean) (SweepResult :type "HitResult Structure (by ref)"))
  (bind (_currentmonsterstat_basehp _currentmonsterstat_basedamage) (break `/Game/Blueprints/Data/Structure/S_MonsterStat` (`self.CurrentMonsterStat`)))
  (if (`self.ActorHasTag` OtherActor "Player")
    (if (not (`KismetArrayLibrary.Array_Contains` (`self.HitActors`) OtherActor))
      (`GameplayStatics.ApplyDamage` OtherActor _currentmonsterstat_basedamage (`self.AIC_Monster`) self "/Script/Engine.DamageType")
      (`KismetArrayLibrary.Array_Add` (`self.HitActors`) OtherActor))))

(fn `OnEndAttack`
  (`PrimitiveComponent.SetCollisionEnabled` (`self.AttackCollision`) "NoCollision"))

(fn `OnStartAttack`
  (`PrimitiveComponent.SetCollisionEnabled` (`self.AttackCollision`) "QueryAndPhysics")
  (`KismetArrayLibrary.Array_Clear` (`self.HitActors`)))

(fn `UserConstructionScript`
  (`parent.UserConstructionScript`))